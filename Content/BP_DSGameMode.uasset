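; BP_DSGameMode is a game mode that restarts the level when the player dies.
; Each Tick it casts player pawn 0 to BP_PlayableCharacter and reads a float attribute from it, which is presumably health.
; When that value reaches zero or below, it disables input, sets a RestartingLevel guard, waits three seconds, and opens DSTestMap.
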(event `self.ReceiveTick`
  (params (DeltaSeconds :type "Float (single-precision)"))
  (bind _asbp_playable_character (cast `/Game/Blueprints/BP_PlayableCharacter` (`GameplayStatics.GetPlayerPawn` 0)))
  (bind (_bsuccessfullyfoundattribute _returnvalue) (`AbilitySystemBlueprintLibrary.GetFloatAttribute` _asbp_playable_character (struct :`AttributeName` "Health" :`Attribute` "/Script/DS.DSBaseCharacterAttributeSet:Health" :`AttributeOwner` "/Script/CoreUObject.Class'/Script/DS.DSBaseCharacterAttributeSet'")))
  (if (and _bsuccessfullyfoundattribute (<= _returnvalue 0.0) (not (`self.bRestartingLevel`)))
    (`self.DisableInput` _asbp_playable_character null)
    (set `self.bRestartingLevel` true)
    (`KismetSystemLibrary.Delay` 3.0)
    (`GameplayStatics.OpenLevelBySoftObjectPtr` "/Game/Map/DSTestMap.DSTestMap")))

(fn `UserConstructionScript`)