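; BP_EnemyAI is an enemy that chases and attacks a perceived actor and leaves a potion when destroyed.
; Perception updates store the actor as Player; Tick moves toward it within range unless actions are blocked, then activates GA_HeavyAttack through GAS on arrival.
; On destruction, it spawns BP_Potion at a line trace hit, with the trace end computed by multiplying its location, not offsetting it.
; An event feeds health percentage to its widget bar.
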(event `self.ReceiveBeginPlay`
  (add `self.OnDestroyed` (delegate `OnDestroyed_Event`)))

(event `OnDestroyed_Event` :!signature `self.OnDestroyed`
  (params (DestroyedActor :type "Actor Object Reference"))
  (bind _returnvalue (`self.K2_GetActorLocation`))
  (bind _outhit (`KismetSystemLibrary.LineTraceSingle` _returnvalue (* _returnvalue (0.0 0.0 -300.0)) "TraceTypeQuery1"))
  (`|SpawnActorFromClass` "/Game/Blueprints/BP_Potion.BP_Potion_C" (`KismetMathLibrary.Conv_VectorToTransform` (`.Location` (`GameplayStatics.BreakHitResult` _outhit))) "Undefined" "MultiplyWithRoot" null null))

(event `self.AIPerception.OnTargetPerceptionUpdated`
  (params (Actor :type "Actor Object Reference") (Stimulus :type "AIStimulus Structure"))
  (set `self.Player` Actor))

(event `self.ReceiveTick`
  (params (DeltaSeconds :type "Float (single-precision)"))
  (bind _player (`self.Player`))
  (`/Engine/EditorBlueprintResources/StandardMacros.IsValid` _player
    (:`Is Valid`
      (if (< (`self.GetDistanceTo` _player) 700.0)
        (if (not (`GameplayTagAssetInterface.HasMatchingGameplayTag` (`AbilitySystemBlueprintLibrary.GetAbilitySystemComponent` null) (struct :`TagName` "State.ActionsBlocked")))
          (`|AIMoveTo` self (`self.K2_GetActorLocation` (`self.Player`)) null 100.0
            (:`OnSuccess`
              (`AbilitySystemComponent.TryActivateAbilityByClass` (`AbilitySystemBlueprintLibrary.GetAbilitySystemComponent` null) "/Game/Blueprints/GAS/GA_HeavyAttack.GA_HeavyAttack_C" true))))))))

(event `self.UpdateHealthBar`
  (params (NewPercentage :type "Float (single-precision)"))
  (bind _aswbp_health_bar (cast `/Game/Blueprints/WBP_HealthBar` (`WidgetComponent.GetWidget` (`self.HealthBar`))))
  (`/Game/Blueprints/WBP_HealthBar.UpdateHealth` _aswbp_health_bar NewPercentage))

(fn `UserConstructionScript`)